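; BP_PawnP38 is a player-controlled P-38 aircraft pawn that constantly flies forward along its facing direction.
; Forward and Right axes pitch and yaw it by Speed and frame delta, and Fire spawns a BP_Rocket at the BPRocket transform.
; On BeginPlay it registers two propeller meshes with BPRotateScene.
; Left Shift writes scaled Speed values to BoostOn and BoostOff, which this graph never reads.
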(event EventBeginPlay
  ;[1 1 1] propeller
  (Utilities|Array|Add (Variables|/Game/Bludprint/BP_RotateScene.BP_RotateScene_C|GetPropeller (Variables|Default|GetBP_RotateScene)) (Variables|Default|GetSM_P38_Propeller))
  (Utilities|Array|Add (Variables|/Game/Bludprint/BP_RotateScene.BP_RotateScene_C|GetPropeller (Variables|Default|GetBP_RotateScene)) (Variables|Default|GetSM_P38_Propeller1)))

(event EventTick
  (params (DeltaSeconds :type Float%20%28single-precision%29))
  ;[1 1 1] moveforward
  (Pawn|Input|AddMovementInput (Transformation|GetActorForwardVector) 1.0 false))

(event Input|ActionEvents|InputActionFire
  (params (Key :type Key%20Structure :default "None"))
  ;[1 1 1] attack
  (:Pressed
    (Game|SpawnActorfromClass "/Game/Bludprint/BP_Rocket.BP_Rocket_C" (Transformation|GetWorldTransform (Variables|Default|GetBP_Rocket)) "Undefined" "MultiplyWithRoot" 0 0)))

(event Input|AxisEvents|InputAxisForward
  (params (AxisValue :type Float%20%28single-precision%29))
  ;[1 1 1] move
  (Transformation|AddActorLocalRotation (Math|Rotator|MakeRotator 0.0 (* AxisValue (Utilities|Time|GetWorldDeltaSeconds) (Variables|Default|GetSpeed)) 0.0) false false))

(event Input|AxisEvents|InputAxisRight
  (params (AxisValue :type Float%20%28single-precision%29))
  ;[1 1 1] move
  (Transformation|AddActorLocalRotation (Math|Rotator|MakeRotator 0.0 0.0 (* AxisValue (Utilities|Time|GetWorldDeltaSeconds) (Variables|Default|GetSpeed))) false false))

(event Input|KeyboardEvents|LeftShift
  (params (Key :type Key%20Structure :default "None"))
  ;[1 1 1] boost
  (:Pressed
    (Variables|Default|SetBoostOn (* (Variables|Default|GetSpeed) 2.0)))
  (:Released
    (Variables|Default|SetBoostOff (* (Variables|Default|GetSpeed) -2.0))))

(fn ConstructionScript)